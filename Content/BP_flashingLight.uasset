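; BP_flashingLight is an actor Blueprint that smoothly pulses the intensity of a light on its owning actor.
; At BeginPlay it caches the owner's first LightComponent and sets it to minimum intensity.
; Each Tick advances a timer that wraps at PulseRate, which acts as the cycle length in seconds, and maps a sine of that phase between the minimum and maximum intensities.
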(event `self.ReceiveBeginPlay`
  (bind _output_get (set `self.Control Light` (`self.GetComponentByClass` (`self.GetOwner`) "/Script/Engine.LightComponent")))
  (`/Engine/EditorBlueprintResources/StandardMacros.IsValid` _output_get
    (:`Is Valid`
      (`LightComponent.SetIntensity` _output_get (`self.Min Light Intensity`)))))

(event `self.ReceiveTick`
  (params (DeltaSeconds :type "Float (single-precision)"))
  (bind _pulse_rate (`self.Pulse Rate`))
  (bind _output_get (set `self.Progress time` (mod (+ DeltaSeconds (`self.Progress time`)) _pulse_rate)))
  (bind _output_get_2 (set `self.Progress Alpha` (/ _output_get _pulse_rate)))
  (bind _control_light (`self.Control Light`)
    (:`then`
      (`LightComponent.SetIntensity` _control_light (`KismetMathLibrary.MapRangeClamped` (`KismetMathLibrary.DegSin` (* _output_get_2 360.0)) -1.0 1.0 (`self.Min Light Intensity`) (`self.Max Light Intensity`))))
    (:`else`)))

(fn `UserConstructionScript`)